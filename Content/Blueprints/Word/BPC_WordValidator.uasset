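; Component that manages a resizable row of card zones in the word game and finds the words their cards can spell.
; Zones are rebuilt as UI widgets in three sizes, discarding held cards on resize.
; When all zones are filled, validation recursively combines each card's active-face letters, treating "-" as blank, and keeps Dictionary DataTable row matches.
; Each match is scored via GameMode LetterRules and shown as a button; consuming discards the cards.
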(event EventBeginPlay
  (bind _asbp_loop_hero_gm (Utilities|Casting|CastToBP_LoopHero_GM (Game|GetGameMode)))
  (bind _output_get (Variables|Default|SetgameMode _asbp_loop_hero_gm))
  (Variables|/Game/Blueprints/Game/BP_LoopHero_GM.BP_LoopHero_GM_C|Getinterface _output_get :!label _label
    (:then
      (bind _returnvalue (Actor|GetActorOfClass "/Game/Blueprints/Controller/BP_Pawn.BP_Pawn_C"))
      (Variables|Default|Setpawn _returnvalue)
      (CallFunction|ResizeZones (CallFunction|GetZoneCountforSize (Variables|Default|GetcurrentSize))))
    (:else
      (Utilities|FlowControl|DelayUntilNextTick)
      (goto _label))))

(fn GetZoneCountforSize
  (params (size :type EPlayerSize%20Enum :default "NewEnumerator0"))
  (return (Utilities|Select :Index size :NewEnumerator0 (Variables|Default|GetsmallZoneCount) :NewEnumerator1 (Variables|Default|GetnormalZoneCount) :NewEnumerator2 (Variables|Default|GetbigZoneCount))))

(fn CreateZones
  (params (count :type Integer))
  (Utilities|Array|Clear (Variables|Default|Getzones))
  (for _index (range 0 (- count 1))
    (bind _returnvalue (UserInterface|CreateWidget (Variables|Default|GetzonePrefab)))
    (Widget|Panel|AddChild (Variables|/Game/Widgets/WBP_HUD.WBP_HUD_C|GetSlotPanel (Variables|/Game/Blueprints/Game/BP_LoopHero_GM.BP_LoopHero_GM_C|Getinterface (Variables|Default|GetgameMode))) _returnvalue)
    (Utilities|Array|Add (Variables|Default|Getzones) _returnvalue)
    (EventDispatchers|BindEventtoOnZoneChanged _returnvalue (EventDispatchers|CreateEvent :!event Validate))))

(fn ResizeZones
  (params (newCount :type Integer))
  (bind _zones (Variables|Default|Getzones))
  (Utilities|FlowControl|Sequence
    (:then_0
      (if (Utilities|Array|IsNotEmpty _zones)
        (for _array_element _zones
          (Utilities|FlowControl|Sequence
            (:then_0
              (bind _currentcard (Variables|/Game/Widgets/WBP_DropZone.WBP_DropZone_C|GetcurrentCard _array_element)
                (:then
                  (Utilities|Array|Add (LocalVariables|GetexistingCards) _currentcard))
                (:else)))
            (:then_1
              (EventDispatchers|UnbindEventfromOnZoneChanged _array_element (EventDispatchers|CreateEvent :!event Validate))
              (Widget|RemovefromParent _array_element))))))
    (:then_1
      (CallFunction|CreateZones newCount)
      (for _array_element_2 (LocalVariables|GetexistingCards)
        (Default|Discard _array_element_2))
      (CallFunction|Validate))))

(fn Shrink
  (bind _output_get (Variables|Default|SetcurrentSize (Utilities|Select :Index (Variables|Default|GetcurrentSize) :NewEnumerator0 "NewEnumerator0" :NewEnumerator1 "NewEnumerator0" :NewEnumerator2 "NewEnumerator1")))
  (CallFunction|ResizeZones (CallFunction|GetZoneCountforSize _output_get)))

(fn Grow
  (bind _output_get (Variables|Default|SetcurrentSize (Utilities|Select :Index (Variables|Default|GetcurrentSize) :NewEnumerator0 "NewEnumerator1" :NewEnumerator1 "NewEnumerator2" :NewEnumerator2 "NewEnumerator2")))
  (CallFunction|ResizeZones (CallFunction|GetZoneCountforSize _output_get)))

(fn Validate
  (CallFunction|ClearResults)
  (if (CallFunction|AllZonesFilled)
    (bind _results (CallFunction|GetValidWords))
    (bind _output_get (LocalVariables|SetvalidWords _results))
    (for _array_element _output_get
      (CallFunction|SpawnButton _array_element))))

(fn AllZonesFilled
  (for _array_element (Variables|Default|Getzones)
    (if (not (Utilities|IsValid (Variables|/Game/Widgets/WBP_DropZone.WBP_DropZone_C|GetcurrentCard _array_element)))
      (return false)))
  (return true))

(fn GetValidWords
  (for _array_element (Variables|Default|Getzones)
    (Utilities|Array|Add (LocalVariables|GetletterPools) (Utilities|Struct|MakeSPool (select (.isFront (Utilities|Struct|BreakSCardData (Variables|/Game/Widgets/WBP_Card.WBP_Card_C|GetcardData (Variables|/Game/Widgets/WBP_DropZone.WBP_DropZone_C|GetcurrentCard _array_element)))) (.frontFace (Utilities|Struct|BreakSCardData (Variables|/Game/Widgets/WBP_Card.WBP_Card_C|GetcardData (Variables|/Game/Widgets/WBP_DropZone.WBP_DropZone_C|GetcurrentCard _array_element)))) (.backFace (Utilities|Struct|BreakSCardData (Variables|/Game/Widgets/WBP_Card.WBP_Card_C|GetcardData (Variables|/Game/Widgets/WBP_DropZone.WBP_DropZone_C|GetcurrentCard _array_element))))))))
  (Utilities|Array|Clear (Variables|Default|Getresults))
  (CallFunction|GenerateCombinations (LocalVariables|GetletterPools))
  (Development|PrintString (Utilities|String|ToString(Integer) (Utilities|Array|Length (Variables|Default|Getresults))))
  (return (Variables|Default|Getresults)))

(fn GenerateCombinations
  (params (pools :type Array%20of%20S%20Pool%20Structures) (index :type Integer) (current :type String))
  (bind _returnvalue (+ index 1))
  (Utilities|FlowControl|Sequence
    (:then_0
      (if (== index (Utilities|Array|Length pools))
        (Utilities|FlowControl|Sequence
          (:then_0
            (if (CallFunction|IsValid current)
              (Utilities|Array|Add (Variables|Default|Getresults) (Utilities|Struct|MakeSWordResult current (CallFunction|ComputeScore current)))))
          (:then_1
            (return)))))
    (:then_1
      (for _array_element (.letters (Utilities|Array|Get(acopy) pools index))
        (if (Utilities|Enum|Equal(Enum) _array_element "-")
          (CallFunction|GenerateCombinations pools _returnvalue current)
          (else
            (CallFunction|GenerateCombinations pools _returnvalue (Utilities|String|Append current _array_element))))))))

(fn ComputeScore
  (params (word :type String))
  (bind _wordscore (Default|ComputeWordScore (Variables|/Game/Blueprints/Game/BP_LoopHero_GM.BP_LoopHero_GM_C|GetLetterRules (Variables|Default|GetgameMode)) word))
  (return _wordscore))

(fn SpawnButton
  (params (result :type S%20Word%20Result%20Structure))
  (bind _returnvalue (UserInterface|CreateWidget (Variables|Default|GetwordButtonPrefab)))
  (Widget|Panel|AddChild (Variables|/Game/Widgets/WBP_HUD.WBP_HUD_C|GetWordPanel (Variables|/Game/Blueprints/Game/BP_LoopHero_GM.BP_LoopHero_GM_C|Getinterface (Variables|Default|GetgameMode))) _returnvalue)
  (Default|Setup _returnvalue result (Variables|Default|Getpawn) self false)
  (Utilities|Array|Add (Variables|Default|GetspawnedButtons) _returnvalue))

(fn CreateConsumedPanel
  (return false))

(fn ClearResults
  (bind _spawnedbuttons (Variables|Default|GetspawnedButtons))
  (for _array_element _spawnedbuttons
    (Widget|RemovefromParent _array_element))
  (Utilities|Array|Clear _spawnedbuttons))

(fn ConsumeCards
  (CallFunction|ClearResults)
  (for _array_element (Variables|Default|Getzones)
    (bind _currentcard (Variables|/Game/Widgets/WBP_DropZone.WBP_DropZone_C|GetcurrentCard _array_element)
      (:then
        (Default|Discard _currentcard))
      (:else))))

(fn HandleWordHovered
  (params (word :type String)))

(fn ClearPulses)

(fn IsValid
  (params (word :type String))
  (bind _outrownames (DataTable|GetDataTableRowNames (Variables|Default|Getdictionary)))
  (return (Utilities|Array|ContainsItem _outrownames (Utilities|String|StringToName (Class|KismetStringLibrary|ToUpper word)))))