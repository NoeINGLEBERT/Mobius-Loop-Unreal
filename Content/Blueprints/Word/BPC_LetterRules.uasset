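; BPC_LetterRules is a Blueprint that supplies letter-based scoring rules for words.
; GetLetterScore looks up a single character's value in the LetterScores map.
; ComputeWordScore splits a word into characters and returns the sum of their letter scores.
; The event graph holds only disabled BeginPlay and Tick stubs, so all logic lives in these two functions.
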(event EventBeginPlay)

(event EventTick
  (params (DeltaSeconds :type Float%20%28single-precision%29)))

(fn GetLetterScore
  (params (c :type String))
  (return (.Value (Utilities|Map|Find (Variables|Default|GetLetterScores) c))))

(fn ComputeWordScore
  (params (word :type String))
  (for _array_element (Utilities|String|GetCharacterArrayfromString word)
    (LocalVariables|Setscore (+ (LocalVariables|Getscore) (CallFunction|GetLetterScore _array_element))))
  (return (LocalVariables|Getscore)))