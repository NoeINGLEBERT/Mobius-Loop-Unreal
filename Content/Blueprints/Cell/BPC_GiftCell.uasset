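; BPC_GiftCell is a cell effect that gifts the player extra cards when activated.
; ActivateEffect loops a few times, asking the game mode's DeckGenerator for a card with a fixed argument and adding it to the DeckManager's DrawPile.
; The deck UI refreshes after each added card.
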(event EventBeginPlay
  (|CallParentFunction) ; This node is disabled and will not be called.\nDrag off pins to build functionality.
)

(event EventTick
  (params (DeltaSeconds :type Float%20%28single-precision%29))
  (|CallParentFunction DeltaSeconds) ; This node is disabled and will not be called.\nDrag off pins to build functionality.
)

(event EventActivateEffect
  (params (pawn :type BP%20Pawn%20Object%20Reference))
  (bind _gamemoderef (Variables|Default|GetgameModeRef))
  (bind _deckmanager (Variables|/Game/Blueprints/Game/BP_LoopHero_GM.BP_LoopHero_GM_C|GetDeckManager _gamemoderef))
  (for _index (range 0 2)
    (Utilities|Array|Add (Variables|/Game/Blueprints/Card/BPC_DeckManager.BPC_DeckManager_C|GetdrawPile _deckmanager) (Default|GenerateCard (Variables|/Game/Blueprints/Game/BP_LoopHero_GM.BP_LoopHero_GM_C|GetDeckGenerator _gamemoderef) 10))
    (Default|UpdateUI _deckmanager)))