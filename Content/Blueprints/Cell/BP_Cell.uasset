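; BP_Cell is a cell that holds one effect for even laps and another for odd laps.
; Setter and getter functions write or read the effect in the slot chosen by an EvenLap flag.
; ActivateCell picks the effect matching the lap parity and, if it is valid, sends it ActivateEffectMessage with the given pawn.
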(event EventBeginPlay)

(fn ConstructionScript)

(fn ActivateCell
  (params (pawn :type BP%20Pawn%20Object%20Reference) (evenLap :type Boolean))
  (bind _evenlapeffect (Variables|Default|GetevenLapEffect))
  (bind _oddlapeffect (Variables|Default|GetoddLapEffect))
  (bind _returnvalue (select evenLap _evenlapeffect _oddlapeffect))
  (Utilities|IsValid _returnvalue
    (:Is%20Valid
      (Class|BPICellEffect|ActivateEffect(Message) _returnvalue pawn))))

(fn GetEffect
  (params (evenLap :type Boolean))
  (return (select evenLap (Variables|Default|GetevenLapEffect) (Variables|Default|GetoddLapEffect))))

(fn SetEffect
  (params (evenLap :type Boolean) (effect :type BPC%20Cell%20Effect%20Object%20Reference))
  (if evenLap
    (Variables|Default|SetevenLapEffect effect)
    (else
      (Variables|Default|SetoddLapEffect effect))))