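; Board-game pawn for a character, which hops along board cells or swaps to the cell offset by the board's cell count.
; Queued Move and Swap commands run one at a time through a gate, and a Swap queued behind another Swap cancels both.
; Timelines animate sine-arc hops and linear swaps, then save the cell index to the GameInstance.
; Finishing a move also triggers the landing cell's effect component.
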(event Custom|ExecuteQueue
  (bind _commandqueue (Variables|Default|GetcommandQueue))
  (Variables|Default|SetisExecuting true)
  (if (Utilities|Array|IsNotEmpty (Variables|Default|GetcommandQueue))
    (Utilities|FlowControl|Sequence
      (:then_0
        (Utilities|FlowControl|Gate false :!label _label
          (:Exit
            (Utilities|FlowControl|Sequence
              (:then_0
                (bind _output_get (Variables|Default|SetcurrentCommand (Utilities|Array|Get(acopy) _commandqueue)))
                (Utilities|Array|RemoveIndex _commandqueue)
                (switch Utilities|FlowControl|Switch|SwitchonEPawnCommandType (.type (Utilities|Struct|BreakSPawnCommand _output_get))
                  (:NewEnumerator0
                    (CallFunction|MoveAnimated (.amount (Utilities|Struct|BreakSPawnCommand _output_get)) (.duration (Utilities|Struct|BreakSPawnCommand _output_get))))
                  (:NewEnumerator1
                    (CallFunction|SwapAnimated))))
              (:then_1
                (goto _label Close))))))
      (:then_1
        (Utilities|FlowControl|DelayUntilNextTick)
        (CallFunction|ExecuteQueue)))
    (else
      (Variables|Default|SetisExecuting false))))

(event Custom|CommandCompleted
  (bind _commandqueue (Variables|Default|GetcommandQueue))
  (Utilities|FlowControl|Gate false) ; enters at Open
)

(event Custom|MoveAnimated
  (params (cellCount :type Integer) (totalDuration :type Float%20%28double-precision%29))
  (bind _character (Variables|Default|Getcharacter))
  (bind _gameinstance (Variables|Default|GetgameInstance))
  (bind _characterdata (Variables|/Game/Blueprints/Game/BP_LoopHero_GI.BP_LoopHero_GI_C|GetCharacterData _gameinstance))
  (bind _value (Utilities|Map|Find _characterdata _character))
  (CallFunction|Hop (.cellindex _value) (+ (.cellindex _value) 1) (/ totalDuration cellCount) cellCount))

(event Custom|Hop
  (params (fromIndex :type Integer) (toIndex :type Integer) (duration :type Float%20%28double-precision%29) (hopLeft :type Integer))
  (bind _returnvalue (- hopLeft 1))
  (bind _board (Variables|Default|Getboard))
  (bind _gameinstance (Variables|Default|GetgameInstance))
  (bind _character (Variables|Default|Getcharacter))
  (bind _board_2 (Variables|Default|Getboard))
  (bind (_position _rotation) (Default|GetCellTransform _board_2 toIndex))
  (bind (_position_2 _rotation_2) (Default|GetCellTransform _board fromIndex))
  (bind _characterdata (Variables|/Game/Blueprints/Game/BP_LoopHero_GI.BP_LoopHero_GI_C|GetCharacterData _gameinstance))
  (Components|Timeline|SetPlayRate (Variables|Default|GetHopTimeline) (/ 1.0 duration))
  (Variables|Default|SetstartTransform (Math|Transform|MakeTransform _position_2 _rotation_2 "1.000000,1.000000,1.000000"))
  (Variables|Default|SetendTransform (Math|Transform|MakeTransform _position _rotation "1.000000,1.000000,1.000000"))
  (bind _t (Timeline|HopTimeline PlayFromStart)
    (:Update
      (bind _output_get (Variables|Default|SetyOffset (* (Math|Vector|GetUpVector (.rotation (Variables|Default|GetstartTransform))) (* (Math|Trig|Sin(Radians) (* _t (Math|Trig|GetPI))) (Variables|Default|Getheight)))))
      (Transformation|SetActorLocationAndRotation (+ _output_get (.Location (Math|Transform|BreakTransform (Math|Transform|Lerp(Transform) (Variables|Default|GetstartTransform) (Variables|Default|GetendTransform) _t)))) (.Rotation (Math|Transform|BreakTransform (Math|Transform|Lerp(Transform) (Variables|Default|GetstartTransform) (Variables|Default|GetendTransform) _t)))))
    (:Finished
      (if (> _returnvalue 0)
        (CallFunction|Hop (+ fromIndex 1) (+ toIndex 1) duration _returnvalue)
        (else
          (Utilities|Map|Remove _characterdata _character)
          (Utilities|Map|Add _characterdata _character (Utilities|Struct|MakeSCharacterData toIndex))
          (CallFunction|CommandCompleted)
          (bind _returnvalue_2 (Actor|GetActorOfClass "/Game/Blueprints/Cell/BP_Board.BP_Board_C"))
          (Class|BPICellEffect|ActivateEffect(Message) (Actor|GetComponentbyClass (Default|GetCell _returnvalue_2 toIndex) "/Game/Blueprints/Cell/BPC_CellEffect.BPC_CellEffect_C") self))))))

(event Custom|SwapAnimated
  (bind _gameinstance (Variables|Default|GetgameInstance))
  (bind _character (Variables|Default|Getcharacter))
  (bind _gameinstance_2 (Variables|Default|GetgameInstance))
  (bind _character_2 (Variables|Default|Getcharacter))
  (bind _board (Variables|Default|Getboard))
  (bind _characterdata (Variables|/Game/Blueprints/Game/BP_LoopHero_GI.BP_LoopHero_GI_C|GetCharacterData _gameinstance_2))
  (bind _characterdata_2 (Variables|/Game/Blueprints/Game/BP_LoopHero_GI.BP_LoopHero_GI_C|GetCharacterData _gameinstance))
  (bind _value (Utilities|Map|Find _characterdata _character))
  (bind (_position _rotation) (Default|GetCellTransform _board (.cellindex _value)))
  (Variables|Default|SetstartTransform (Math|Transform|MakeTransform _position _rotation "1.000000,1.000000,1.000000"))
  (bind _output_get (Variables|Default|SetswapIndex (+ (.cellindex _value) (Variables|/Game/Blueprints/Cell/BP_Board.BP_Board_C|GetcellNumber _board))))
  (Variables|Default|SetendTransform (Math|Transform|MakeTransform (.position (Default|GetCellTransform _board _output_get)) (.rotation (Default|GetCellTransform _board _output_get)) "1.000000,1.000000,1.000000"))
  (bind _t (Timeline|SwapTimeline PlayFromStart)
    (:Update
      (Transformation|SetActorTransform (Math|Transform|Lerp(Transform) (Variables|Default|GetstartTransform) (Variables|Default|GetendTransform) _t)))
    (:Finished
      (Utilities|Map|Remove _characterdata_2 _character_2)
      (Utilities|Map|Add _characterdata_2 _character_2 (Utilities|Struct|MakeSCharacterData (Variables|Default|GetswapIndex)))
      (CallFunction|CommandCompleted))))

(event EventBeginPlay
  (bind _asbp_loop_hero_gi (Utilities|Casting|CastToBP_LoopHero_GI (Game|GetGameInstance)))
  (bind _output_get (Variables|Default|SetgameInstance _asbp_loop_hero_gi))
  (CallFunction|SnaptoCell (.cellindex (.Value (Utilities|Map|Find (Variables|/Game/Blueprints/Game/BP_LoopHero_GI.BP_LoopHero_GI_C|GetCharacterData _output_get) (Variables|Default|Getcharacter))))))

(fn ConstructionScript)

(fn IsIdle
  (return (and (not (Variables|Default|GetisExecuting)) (Utilities|Array|IsEmpty (Variables|Default|GetcommandQueue)))))

(fn MoveUpCells
  (params (cellCount :type Integer) (duration :type Float%20%28double-precision%29))
  (CallFunction|Enqueue (Utilities|Struct|MakeSPawnCommand "NewEnumerator0" cellCount duration)))

(fn Swap
  (CallFunction|Enqueue (Utilities|Struct|MakeSPawnCommand "NewEnumerator1" 0 0.5)))

(fn Enqueue
  (params (command :type S%20Pawn%20Command%20Structure))
  (bind _commandqueue (Variables|Default|GetcommandQueue))
  (bind _commandqueue_2 (Variables|Default|GetcommandQueue))
  (Utilities|FlowControl|Sequence
    (:then_0
      (if (and (Utilities|Enum|Equal(Enum) (Utilities|Struct|BreakSPawnCommand command) "NewEnumerator1") (Utilities|Array|IsNotEmpty (Variables|Default|GetcommandQueue)))
        (bind _output_get (LocalVariables|SetlastCommand (Utilities|Array|Get(acopy) _commandqueue (Utilities|Array|LastIndex _commandqueue))))
        (if (Utilities|Enum|Equal(Enum) (.type _output_get) "NewEnumerator1")
          (Utilities|Array|RemoveIndex _commandqueue_2 (Utilities|Array|LastIndex _commandqueue_2))
          (return))))
    (:then_1
      (Utilities|Array|Add (Variables|Default|GetcommandQueue) command)
      (if (not (Variables|Default|GetisExecuting))
        (CallFunction|ExecuteQueue)))))

(fn SnaptoCell
  (params (cellIndex :type Integer))
  (bind _board (Variables|Default|Getboard))
  (bind (_position _rotation) (Default|GetCellTransform _board cellIndex))
  (Transformation|SetActorLocationAndRotation _position _rotation))