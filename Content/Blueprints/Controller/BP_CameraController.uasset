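; BP_CameraController is an orbit camera for the LoopHero game mode, always facing the world origin.
; Holding left mouse hides the cursor and opens a Tick gate that drives yaw and clamped pitch, while zoom input adjusts clamped distance.
; Both rebuild the actor transform from rotation and distance.
; Releasing the button closes the gate, restores cursor and Game-and-UI input, and notifies the game mode that card dragging has ended.
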(event EventBeginPlay
  (Variables|Default|Setdistance (Variables|Default|GetmaxDistance))
  (CallFunction|UpdateCameraTransform)
  (bind _asbp_loop_hero_gm (Utilities|Casting|CastToBP_LoopHero_GM (Game|GetGameMode)))
  (Variables|Default|SetgameMode _asbp_loop_hero_gm))

(event EventTick
  (params (DeltaSeconds :type Float%20%28single-precision%29))
  (CallFunction|HandleZoom)
  (Utilities|FlowControl|Gate true
    (:Exit
      (CallFunction|HandleRotation))))

(event Input|MouseEvents|LeftMouseButton
  (params (Key :type Key%20Structure :default "None"))
  (bind _returnvalue (Game|GetPlayerController 0))
  (bind _gamemode (Variables|Default|GetgameMode))
  (:Pressed
    (Utilities|FlowControl|DelayUntilNextTick)
    (Variables|/Script/Engine.PlayerController|SetbShowMouseCursor _returnvalue false)
    (Variables|Default|Setrotating true)
    (Utilities|FlowControl|Gate true) ; enters at Open
  )
  (:Released
    (Default|OnEndDragCard _gamemode)
    (Variables|/Script/Engine.PlayerController|SetbShowMouseCursor _returnvalue true)
    (Input|SetInputModeGameandUI (Game|GetPlayerController 0) (Variables|/Game/Blueprints/Game/BP_LoopHero_GM.BP_LoopHero_GM_C|Getinterface _gamemode) "DoNotLock" true false)
    (Variables|Default|Setrotating false)
    (Utilities|FlowControl|Gate true) ; enters at Close
  ))

(fn ConstructionScript)

(fn HandleRotation
  (bind _pitchlimits (Variables|Default|GetpitchLimits))
  (Variables|Default|Setyaw (+ (Variables|Default|Getyaw) (* (Class|Actor|GetInputAxisKeyValue) (Variables|Default|GetyawSpeed) (Utilities|Time|GetWorldDeltaSeconds))))
  (Variables|Default|Setpitch (Math|Float|Clamp(Float) (+ (Variables|Default|Getpitch) (* (Class|Actor|GetInputAxisKeyValue) (Variables|Default|GetpitchSpeed) (Utilities|Time|GetWorldDeltaSeconds))) (.x _pitchlimits) (.y _pitchlimits)))
  (CallFunction|UpdateCameraTransform))

(fn HandleZoom
  (bind _returnvalue (Class|Actor|GetInputAxisKeyValue))
  (if (> (Math|Float|Absolute(Float) _returnvalue) 0.01)
    (Variables|Default|Setdistance (Math|Float|Clamp(Float) (- (Variables|Default|Getdistance) (* _returnvalue (Variables|Default|GetzoomSpeed))) (Variables|Default|GetminDistance) (Variables|Default|GetmaxDistance)))
    (CallFunction|UpdateCameraTransform)))

(fn UpdateCameraTransform
  (bind _yaw (Variables|Default|Getyaw))
  (bind _pitch (Variables|Default|Getpitch))
  (bind _returnvalue (Math|Rotator|MakeRotator 0.0 _pitch _yaw))
  (Transformation|SetActorLocationAndRotation (* (Math|Vector|GetForwardVector _returnvalue) (Variables|Default|Getdistance) -1.0) _returnvalue))