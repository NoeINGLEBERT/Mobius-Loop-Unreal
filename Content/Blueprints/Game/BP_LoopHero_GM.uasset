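; BP_LoopHero_GM is the game mode for a Loop Hero card game, creating the HUD and resolving card drags.
; BeginPlay creates WBP_HUD, stores it as Interface and adds it to the viewport.
; OnEndDragCard hands the dragged card to a valid hovered drop zone and clears the reference.
; Otherwise, after a one-tick delay, it returns any card not marked as dropped in a zone to the hand.
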(event Custom|OnEndDragCard
  (Utilities|FlowControl|Sequence
    (:then_0
      (bind _hovereddropzone (Variables|Default|GethoveredDropZone)
        (:then
          (Default|SetCard _hovereddropzone (Variables|Default|GetdraggedCard))
          (Variables|Default|SetdraggedCard 0))
        (:else)))
    (:then_1
      (Utilities|FlowControl|DelayUntilNextTick)
      (bind _draggedcard (Variables|Default|GetdraggedCard)
        (:then
          (if (not (Variables|/Game/Widgets/WBP_Card.WBP_Card_C|GetdroppedInZone _draggedcard))
            (Default|ReturntoHand _draggedcard)
            (Variables|Default|SetdraggedCard 0)))
        (:else)))))

(event EventBeginPlay
  (bind _returnvalue (UserInterface|CreateWidget "/Game/Widgets/WBP_HUD.WBP_HUD_C" (Game|GetPlayerController 0)))
  (bind _output_get (Variables|Default|Setinterface _returnvalue))
  (UserInterface|Viewport|AddtoViewport _output_get 0))

(fn ConstructionScript)