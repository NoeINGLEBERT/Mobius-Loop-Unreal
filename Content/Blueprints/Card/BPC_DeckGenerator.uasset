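; Component that generates the deck of double-sided letter cards and stores it on the game instance.
; BeginPlay expands Scrabble letter counts into a weighted pool; GenerateDeck builds each card from it toward a target point total.
; GenerateCard uses a safety-capped loop, adding unrepeated letters to random sides within score and length limits, with "-" as filler.
; Each card gets opposite-coloured suits on its two faces and a random facing.
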(event EventBeginPlay
  (CallFunction|InitScrabbleLetters)
  (bind _asbp_loop_hero_gi (Utilities|Casting|CastToBP_LoopHero_GI (Game|GetGameInstance)))
  (Variables|Default|SetgameInstance _asbp_loop_hero_gi)
  (bind _asbp_loop_hero_gm (Utilities|Casting|CastToBP_LoopHero_GM (Game|GetGameMode)))
  (Variables|Default|SetgameMode _asbp_loop_hero_gm))

(fn GenerateDeck
  (Variables|Default|GetgameInstance
    (:then
      (for _index (range 0 (- (Variables|Default|GetdeckSize) 1))
        (Utilities|Array|Add (LocalVariables|Getcards) (CallFunction|GenerateCard (Variables|Default|GetcardTargetPoints))))
      (Variables|/Game/Blueprints/Game/BP_LoopHero_GI.BP_LoopHero_GI_C|SetDeck (Variables|Default|GetgameInstance) (LocalVariables|Getcards)))
    (:else)))

(fn InitScrabbleLetters
  (Utilities|Array|Clear (Variables|Default|GetweightedLetterPool))
  (for _array_element (Variables|Default|GetscrabbleLetters)
    (for _index (range 1 (.count _array_element))
      (Utilities|Array|Add (Variables|Default|GetweightedLetterPool) (.letter _array_element)))))

(fn GenerateCard
  (params (targetPoints :type Integer))
  (bind _front (LocalVariables|Getfront))
  (bind _validletters (LocalVariables|GetvalidLetters))
  (bind _front_2 (LocalVariables|Getfront))
  (bind _outitem (Utilities|Array|Random _validletters))
  (while (> (LocalVariables|Getsafety) 0)
    (Math|Integer|DecrementInt (LocalVariables|Getsafety)
      (:%20%20
        (LocalVariables|SettotalPoints (+ (LocalVariables|GetfrontPoints) (LocalVariables|GetbackPoints)))
        (Utilities|FlowControl|Sequence
          (:then_0
            (if (Math|Boolean|ANDBoolean (== (LocalVariables|GettotalPoints) targetPoints) (Utilities|Array|IsNotEmpty (LocalVariables|Getfront)) (Utilities|Array|IsNotEmpty (LocalVariables|Getback)))
              (LocalVariables|Setsafety 0)))
          (:then_1
            (LocalVariables|SetaddToFront (Math|Random|RandomBool))
            (if (not (>= (Utilities|Array|Length (select (LocalVariables|GetaddToFront) (LocalVariables|Getfront) (LocalVariables|Getback))) (Variables|Default|GetmaxLettersPerSide)))
              (Utilities|Array|Clear (LocalVariables|GetvalidLetters))
              (for _array_element (Variables|Default|GetweightedLetterPool)
                (if (not (Math|Boolean|ORBoolean (Utilities|Enum|Equal(Enum) _array_element "-") (Utilities|Array|ContainsItem (LocalVariables|Getback) _array_element) (Utilities|Array|ContainsItem (LocalVariables|Getfront) _array_element) (> (+ (Default|GetLetterScore (Variables|/Game/Blueprints/Game/BP_LoopHero_GM.BP_LoopHero_GM_C|GetLetterRules (Variables|Default|GetgameMode)) _array_element) (LocalVariables|GettotalPoints)) targetPoints)))
                  (Utilities|Array|Add (LocalVariables|GetvalidLetters) _array_element)))
              (Utilities|FlowControl|Sequence
                (:then_0
                  (if (Utilities|Array|IsEmpty (LocalVariables|GetvalidLetters))
                    (Utilities|FlowControl|Sequence
                      (:then_0
                        (if (Utilities|Array|IsEmpty (select (LocalVariables|GetaddToFront) (LocalVariables|Getfront) (LocalVariables|Getback)))
                          (Utilities|Array|Add (select (LocalVariables|GetaddToFront) (LocalVariables|Getfront) (LocalVariables|Getback)) "-")))
                      (:then_1
                        (if (< (LocalVariables|GettotalPoints) targetPoints)
                          (if (and (LocalVariables|GetaddToFront) (Utilities|Array|IsEmpty (LocalVariables|Getback)))
                            (LocalVariables|SetaddToFront false)
                            (elif (and (not (LocalVariables|GetaddToFront)) (Utilities|Array|IsEmpty (LocalVariables|Getfront)))
                              (LocalVariables|SetaddToFront true)))
                          (else
                            (LocalVariables|Setsafety 0)))))))
                (:then_1
                  (bind _output_get (LocalVariables|Setchosen _outitem))
                  (if (Utilities|Enum|NotEqual(Enum) _outitem "")
                    (LocalVariables|Setpoints (Default|GetLetterScore (Variables|/Game/Blueprints/Game/BP_LoopHero_GM.BP_LoopHero_GM_C|GetLetterRules (Variables|Default|GetgameMode)) _output_get))
                    (Utilities|Array|Add (select (LocalVariables|GetaddToFront) (LocalVariables|Getfront) (LocalVariables|Getback)) (LocalVariables|Getchosen))
                    (if (LocalVariables|GetaddToFront)
                      (LocalVariables|SetfrontPoints (+ (LocalVariables|GetfrontPoints) (LocalVariables|Getpoints)))
                      (else
                        (LocalVariables|SetbackPoints (+ (LocalVariables|GetbackPoints) (LocalVariables|Getpoints))))))))))))))
  (Utilities|FlowControl|Sequence
    (:then_0
      (if (Utilities|Array|IsEmpty _front_2)
        (Utilities|Array|Add _front_2 "-")))
    (:then_1
      (if (Utilities|Array|IsEmpty _front)
        (Utilities|Array|Add _front "-")))
    (:then_2
      (LocalVariables|SetfrontIsRed (Math|Random|RandomBool))
      (LocalVariables|SetfrontSuit (select (LocalVariables|GetfrontIsRed) (.OutItem (Utilities|Array|Random (LocalVariables|GetredSuits))) (.OutItem (Utilities|Array|Random (LocalVariables|GetblackSuits)))))
      (LocalVariables|SetbackSuit (select (LocalVariables|GetfrontIsRed) (.OutItem (Utilities|Array|Random (LocalVariables|GetblackSuits))) (.OutItem (Utilities|Array|Random (LocalVariables|GetredSuits)))))
      (LocalVariables|SetisFront (Math|Random|RandomBool))
      (LocalVariables|SetfinalTotal (+ (LocalVariables|GetfrontPoints) (LocalVariables|GetbackPoints)))
      (return (Utilities|Struct|MakeSCardData (LocalVariables|Getfront) (LocalVariables|Getback) (LocalVariables|GetisFront) (LocalVariables|GetfrontSuit) (LocalVariables|GetbackSuit))))))