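; Deck manager component that runs the card draw, hand and discard cycle, triggering defeat when no cards remain to draw.
; Once the interface is valid, it loads and shuffles the GameInstance deck, generating it first if flagged.
; A delayed recursive event draws card widgets toward the WordValidator's zone count, reshuffling discards when the pile empties.
; Discards trigger refills; destroyed cards leave circulation, lowering "Sanity", the displayed draw-plus-discard total.
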(event Custom|RefillHandDelayed
  (bind _gamemode (Variables|Default|GetgameMode))
  (bind _wordvalidator (Variables|/Game/Blueprints/Game/BP_LoopHero_GM.BP_LoopHero_GM_C|GetWordValidator _gamemode))
  (bind _success (CallFunction|DrawOne))
  (if _success
    (Utilities|FlowControl|Delay (Variables|Default|GetdrawInterval))
    (if (< (Utilities|Array|Length (Variables|Default|GethandCards)) (Default|GetZoneCountforSize _wordvalidator (Variables|/Game/Blueprints/Word/BPC_WordValidator.BPC_WordValidator_C|GetcurrentSize _wordvalidator)))
      (CallFunction|RefillHandDelayed))))

(event EventBeginPlay
  (bind _asbp_loop_hero_gm (Utilities|Casting|CastToBP_LoopHero_GM (Game|GetGameMode)))
  (bind _output_get (Variables|Default|SetgameMode _asbp_loop_hero_gm))
  (Variables|/Game/Blueprints/Game/BP_LoopHero_GM.BP_LoopHero_GM_C|Getinterface _output_get :!label _label
    (:then
      (bind _asbp_loop_hero_gi (Utilities|Casting|CastToBP_LoopHero_GI (Game|GetGameInstance)))
      (bind _output_get_2 (Variables|Default|SetgameInstance _asbp_loop_hero_gi))
      (Utilities|FlowControl|Sequence
        (:then_0
          (if (Variables|/Game/Blueprints/Game/BP_LoopHero_GI.BP_LoopHero_GI_C|GetGenerateDeck _output_get_2)
            (Default|GenerateDeck (Variables|/Game/Blueprints/Game/BP_LoopHero_GM.BP_LoopHero_GM_C|GetDeckGenerator (Variables|Default|GetgameMode)))
            (Variables|/Game/Blueprints/Game/BP_LoopHero_GI.BP_LoopHero_GI_C|SetGenerateDeck _output_get_2 false)))
        (:then_1
          (bind _output_get_3 (Variables|Default|SetdrawPile (Variables|/Game/Blueprints/Game/BP_LoopHero_GI.BP_LoopHero_GI_C|GetDeck (Variables|Default|GetgameInstance))))
          (Utilities|Array|Shuffle _output_get_3)
          (CallFunction|UpdateUI)
          (CallFunction|RefillHand))))
    (:else
      (Utilities|FlowControl|DelayUntilNextTick)
      (goto _label))))

(fn RefillHand
  (CallFunction|RefillHandDelayed))

(fn DrawOne
  (bind _drawpile (Variables|Default|GetdrawPile))
  (bind _drawpile_2 (Variables|Default|GetdrawPile))
  (bind _gamemode (Variables|Default|GetgameMode))
  (bind _returnvalue (Utilities|Array|IsEmpty _drawpile))
  (bind _interface (Variables|/Game/Blueprints/Game/BP_LoopHero_GM.BP_LoopHero_GM_C|Getinterface _gamemode))
  (bind _hand (Variables|/Game/Widgets/WBP_HUD.WBP_HUD_C|GetHand _interface))
  (Utilities|FlowControl|Sequence
    (:then_0
      (if _returnvalue
        (CallFunction|RefillfromDiscard)))
    (:then_1
      (if _returnvalue
        (CallFunction|GameOver)
        (return false)))
    (:then_2
      (LocalVariables|Setdata (Utilities|Array|Get(acopy) _drawpile_2))
      (Utilities|Array|RemoveIndex _drawpile_2)
      (bind _returnvalue_2 (UserInterface|CreateWidget "/Game/Widgets/WBP_Card.WBP_Card_C" 0 (LocalVariables|Getdata) _hand))
      (LocalVariables|Setcard _returnvalue_2)
      (Widget|Panel|AddChild _hand _returnvalue_2)
      (Utilities|Array|Add (Variables|Default|GethandCards) (LocalVariables|Getcard))
      (Default|PlayDrawAnimation (LocalVariables|Getcard))
      (CallFunction|UpdateUI)
      (return true))))

(fn HandleDiscard
  (params (card :type WBP%20Card%20Object%20Reference))
  (EventDispatchers|UnbindEventfromOnDiscardRequested card (EventDispatchers|CreateEvent :!event HandleDiscard))
  (Utilities|Array|RemoveItem (Variables|Default|GethandCards) card)
  (Utilities|Array|Add (Variables|Default|GetdiscardPile) (Variables|/Game/Widgets/WBP_Card.WBP_Card_C|GetcardData card))
  (Widget|RemovefromParent card)
  (CallFunction|UpdateUI)
  (Default|ClearCard (Variables|/Game/Widgets/WBP_Card.WBP_Card_C|GetdropZone card))
  (CallFunction|RefillHand))

(fn HandleDestroy
  (params (card :type WBP%20Card%20Object%20Reference))
  (EventDispatchers|UnbindEventfromOnDestroyRequested card (EventDispatchers|CreateEvent :!event HandleDestroy))
  (Utilities|Array|RemoveItem (Variables|Default|GethandCards) card)
  (CallFunction|UpdateUI)
  (Widget|RemovefromParent card)
  (Default|ClearCard (Variables|/Game/Widgets/WBP_Card.WBP_Card_C|GetdropZone card)))

(fn RefillfromDiscard
  (Utilities|FlowControl|Sequence
    (:then_0
      (if (Utilities|Array|IsEmpty (Variables|Default|GetdiscardPile))
        (return)))
    (:then_1
      (Utilities|Array|AppendArray (Variables|Default|GetdrawPile) (Variables|Default|GetdiscardPile))
      (Utilities|Array|Clear (Variables|Default|GetdiscardPile))
      (Utilities|Array|Shuffle (Variables|Default|GetdrawPile))
      (CallFunction|UpdateUI))))

(fn UpdateUI
  (bind _gamemode (Variables|Default|GetgameMode))
  (bind _interface (Variables|/Game/Blueprints/Game/BP_LoopHero_GM.BP_LoopHero_GM_C|Getinterface _gamemode))
  (bind _sanitytext (Variables|/Game/Widgets/WBP_HUD.WBP_HUD_C|GetSanityText _interface))
  (LocalVariables|SetdeckCount (Utilities|Array|Length (Variables|Default|GetdrawPile)))
  (LocalVariables|SetdiscardCount (Utilities|Array|Length (Variables|Default|GetdiscardPile)))
  (LocalVariables|Setsanity (+ (LocalVariables|GetdeckCount) (LocalVariables|GetdiscardCount)))
  (Variables|/Script/UMG.TextBlock|SetText (Variables|/Game/Widgets/WBP_HUD.WBP_HUD_C|GetDeckText _interface) (Utilities|Text|ToText(Integer) (LocalVariables|GetdeckCount)))
  (Variables|/Script/UMG.TextBlock|SetText (Variables|/Game/Widgets/WBP_HUD.WBP_HUD_C|GetDiscardText _interface) (Utilities|Text|ToText(Integer) (LocalVariables|GetdiscardCount)))
  (Variables|/Script/UMG.TextBlock|SetText _sanitytext (Utilities|Text|ToText(String) (Utilities|String|Append (Utilities|String|ToString(Integer) (LocalVariables|Getsanity)) " cards left")))
  (Appearance|SetColorandOpacity _sanitytext (select (> (LocalVariables|Getsanity) 10) (Utilities|Struct|MakeSlateColor "(R=1.000000,G=1.000000,B=1.000000,A=1.000000)") (Utilities|Struct|MakeSlateColor "(R=1.000000,G=0.000000,B=0.000000,A=1.000000)")) :!class /Script/UMG.TextBlock))

(fn GameOver
  (Default|TriggerDefeat (Variables|/Game/Blueprints/Game/BP_LoopHero_GM.BP_LoopHero_GM_C|GetGameStateManager (Variables|Default|GetgameMode))))