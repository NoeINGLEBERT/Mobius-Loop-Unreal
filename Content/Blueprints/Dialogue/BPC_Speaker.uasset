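; Speaker component that links a dialogue character to the game mode's DialogueManager.
; On BeginPlay it caches BP_LoopHero_GM, retries each tick until the manager is valid, then registers itself in the Speakers map under its Character key.
; DisplayDialogue passes the dialogue text and itself to the manager, then sets itself as the current speaker.
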(event EventBeginPlay
  (bind _asbp_loop_hero_gm (Utilities|Casting|CastToBP_LoopHero_GM (Game|GetGameMode)))
  (bind _output_get (Variables|Default|SetgameMode _asbp_loop_hero_gm))
  (bind _dialoguemanager (Variables|/Game/Blueprints/Game/BP_LoopHero_GM.BP_LoopHero_GM_C|GetDialogueManager _output_get :!label _label)
    (:then
      (Utilities|Map|Add (Variables|/Game/Blueprints/Dialogue/BPC_DialogueManager.BPC_DialogueManager_C|Getspeakers _dialoguemanager) (Variables|Default|GetCharacter) self))
    (:else
      (Utilities|FlowControl|DelayUntilNextTick)
      (goto _label))))

(event EventTick
  (params (DeltaSeconds :type Float%20%28single-precision%29)))

(fn DisplayDialogue
  (params (dialogue :type S%20Dialogue%20Entry%20Structure))
  (bind _self self)
  (bind _gamemode (Variables|Default|GetgameMode))
  (bind _dialoguemanager (Variables|/Game/Blueprints/Game/BP_LoopHero_GM.BP_LoopHero_GM_C|GetDialogueManager _gamemode))
  (bind _output_get (Variables|Default|Setdialogue dialogue))
  (Default|DisplayDialogue _dialoguemanager (.dialogueText (Utilities|Struct|BreakSDialogueEntry _output_get)) _self)
  (Variables|/Game/Blueprints/Dialogue/BPC_DialogueManager.BPC_DialogueManager_C|SetcurrentSpeaker _dialoguemanager _self))