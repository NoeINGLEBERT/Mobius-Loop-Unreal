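; Dialogue component that plays data table lines through registered speakers, tracking a starting index and pool of conversations.
; It binds to the GameMode's DialogueManager, where notified events, checked against recorded events, let higher-priority reactions redirect the starting index and pool size.
; Each line notifies its event and displays; choiceless lines bind to skip and advance, while ending lines move through the pool.
; "[EFFECT]" rows with a valid effect divert to an empty PlayEffectAndResume hook.
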(event EventBeginPlay
  (bind _asbp_loop_hero_gm (Utilities|Casting|CastToBP_LoopHero_GM (Game|GetGameMode)))
  (bind _output_get (Variables|Default|SetgameMode _asbp_loop_hero_gm))
  (bind _dialoguemanager (Variables|/Game/Blueprints/Game/BP_LoopHero_GM.BP_LoopHero_GM_C|GetDialogueManager _output_get :!label _label)
    (:then
      (EventDispatchers|BindEventtoOnNotifyEvent _dialoguemanager (EventDispatchers|CreateEvent :!event HandleEventNotify)))
    (:else
      (Utilities|FlowControl|DelayUntilNextTick)
      (goto _label))))

(fn HandleEventNotify
  (params (event :type String))
  (for _array_element (Variables|Default|Getreactions)
    (LocalVariables|SettriggerReaction false)
    (bind _output_get (LocalVariables|SetparsedEvents (Utilities|String|ParseIntoArray event ",")))
    (LocalVariables|SettriggerReaction (Utilities|Array|ContainsItem _output_get event))
    (bind _array_element_2 (Utilities|Array|ForEachLoopwithBreak (LocalVariables|GetparsedEvents) :!label _label)
      (:LoopBody
        (bind _output_get_2 (LocalVariables|SetisIncomingEvent (Utilities|Enum|Equal(Enum) _array_element_2 event)))
        (bind _output_get_3 (LocalVariables|SetexistsInGlobalEvents (Utilities|Array|ContainsItem (Variables|/Game/Blueprints/Dialogue/BPC_DialogueManager.BPC_DialogueManager_C|Getevents (Variables|/Game/Blueprints/Game/BP_LoopHero_GM.BP_LoopHero_GM_C|GetDialogueManager (Variables|Default|GetgameMode))) _array_element_2)))
        (if (not (or _output_get_2 _output_get_3))
          (LocalVariables|SettriggerReaction false)
          (goto _label Break)))
      (:Completed
        (if (LocalVariables|GettriggerReaction)
          (for _array_element_3 (.reactions (Utilities|Struct|BreakSReactionEntry _array_element))
            (if (> (.priority (Utilities|Struct|BreakSReaction _array_element_3)) (Variables|Default|GetlastEventPriority))
              (Variables|Default|SetstartingIndex (.newStartingIndex (Utilities|Struct|BreakSReaction _array_element_3)))
              (Variables|Default|SetdialoguePoolSize (.newDialoguePoolsize (Utilities|Struct|BreakSReaction _array_element_3)))
              (Variables|Default|SetlastEventPriority (.priority (Utilities|Struct|BreakSReaction _array_element_3))))))))))

(fn GetDialoguefromIndex
  (params (index :type Integer))
  (bind _dialoguetable (Variables|Default|GetdialogueTable))
  (bind _outrownames (DataTable|GetDataTableRowNames _dialoguetable))
  (bind _returnvalue (Utilities|GetDataTableRow _dialoguetable (Utilities|Array|Get(acopy) _outrownames index))
    (:then
      (return _returnvalue))))

(fn StartDialogue
  (CallFunction|TryDialogue (Variables|Default|GetstartingIndex)))

(fn TryDialogue
  (params (index :type Integer))
  (Variables|Default|SetcurrentIndex index)
  (CallFunction|PlayDialogue false))

(fn PlayEffectandResume)

(fn PlayDialogue
  (params (isEnd :type Boolean))
  (bind _gamemode (Variables|Default|GetgameMode))
  (bind _currentindex (Variables|Default|GetcurrentIndex))
  (bind _dialoguemanager (Variables|/Game/Blueprints/Game/BP_LoopHero_GM.BP_LoopHero_GM_C|GetDialogueManager _gamemode))
  (if (not isEnd)
    (bind _output_get (LocalVariables|SetcurrentDialogue (CallFunction|GetDialoguefromIndex (Variables|Default|GetcurrentIndex))))
    (Utilities|FlowControl|Sequence
      (:then_0
        (if (Utilities|Enum|Equal(Enum) (.dialogueText (Utilities|Struct|BreakSDialogueEntry _output_get)) "[EFFECT]")
          (Variables|Default|GetdialogueEffect
            (:then
              (CallFunction|PlayEffectandResume)
              (return))
            (:else))))
      (:then_1
        (Variables|/Game/Blueprints/Dialogue/BPC_DialogueManager.BPC_DialogueManager_C|SetcurrentDialogueComponent _dialoguemanager self)
        (bind _output_get_2 (LocalVariables|SetcurrentSpeaker (.Value (Utilities|Map|Find (Variables|/Game/Blueprints/Dialogue/BPC_DialogueManager.BPC_DialogueManager_C|Getspeakers _dialoguemanager) (.speaker (Utilities|Struct|BreakSDialogueEntry _output_get))))))
        (Default|NotifyEvent _dialoguemanager (.eventName (Utilities|Struct|BreakSDialogueEntry _output_get)))
        (Default|DisplayDialogue _output_get_2 (LocalVariables|GetcurrentDialogue))
        (if (.dialogueEnd (Utilities|Struct|BreakSDialogueEntry (LocalVariables|GetcurrentDialogue)))
          (if (> (Variables|Default|GetdialoguePoolSize) 1)
            (Variables|Default|SetstartingIndex (+ _currentindex 1))
            (Math|Integer|DecrementInt (Variables|Default|GetdialoguePoolSize)))
          (elif (not (Utilities|Array|IsNotEmpty (.choicesTexts (Utilities|Struct|BreakSDialogueEntry (LocalVariables|GetcurrentDialogue)))))
            (EventDispatchers|BindEventtoOnDialogueSkipped (Variables|/Game/Blueprints/Game/BP_LoopHero_GM.BP_LoopHero_GM_C|GetDialogueManager (Variables|Default|GetgameMode)) (EventDispatchers|CreateEvent :!event PlayDialogue))
            (Math|Integer|IncrementInt _currentindex)))))))