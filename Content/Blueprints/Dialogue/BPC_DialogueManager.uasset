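; Dialogue manager component that shows a speaker's lines in the game mode's interface widget.
; On BeginPlay it retries each tick until that interface is valid, then binds its skip event.
; Each line appears at once with either a skip button or spawned choice buttons carrying answer indexes; typewriter and input-choice functions are empty stubs.
; Skipping hides the panel when dialogue ends and broadcasts the result; NotifyEvent relays events through a dispatcher.
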(event EventBeginPlay
  (bind _asbp_loop_hero_gm (Utilities|Casting|CastToBP_LoopHero_GM (Game|GetGameMode)))
  (bind _output_get (Variables|Default|SetgameMode _asbp_loop_hero_gm))
  (bind _interface (Variables|/Game/Blueprints/Game/BP_LoopHero_GM.BP_LoopHero_GM_C|Getinterface _output_get :!label _label)
    (:then
      (EventDispatchers|BindEventtoOnSkip _interface (EventDispatchers|CreateEvent :!event SkipDialogue)))
    (:else
      (Utilities|FlowControl|DelayUntilNextTick)
      (goto _label))))

(fn NotifyEvent
  (params (event :type String))
  (Default|CallOnNotifyEvent event))

(fn DisplayDialogue
  (params (DialogueText :type String) (speaker :type BPC%20Speaker%20Object%20Reference))
  (bind _gamemode (Variables|Default|GetgameMode))
  (bind _interface (Variables|/Game/Blueprints/Game/BP_LoopHero_GM.BP_LoopHero_GM_C|Getinterface _gamemode))
  (bind _skipbutton (Variables|/Game/Widgets/WBP_HUD.WBP_HUD_C|GetSkipButton _interface))
  (bind _choicepanel (Variables|/Game/Widgets/WBP_HUD.WBP_HUD_C|GetChoicePanel _interface))
  (Variables|Default|SetcurrentDialogue DialogueText)
  (Variables|Default|SetcurrentSpeaker speaker)
  (Variables|Default|SetdisplayedLetters 0)
  (CallFunction|UpdateText)
  (Variables|/Script/UMG.TextBlock|SetText (Variables|/Game/Widgets/WBP_HUD.WBP_HUD_C|GetCharacterName _interface) (Utilities|Text|ToText(String) (Variables|/Game/Blueprints/Dialogue/BPC_Speaker.BPC_Speaker_C|GetdisplayName speaker)))
  (Widget|SetRenderOpacity _skipbutton 0.0)
  (Widget|SetRenderOpacity _choicepanel 0.0)
  (Widget|SetVisibility _skipbutton "Hidden")
  (for _array_element (Class|PanelWidget|GetAllChildren _choicepanel)
    (Widget|RemovefromParent _array_element))
  (Widget|SetRenderOpacity (Variables|/Game/Widgets/WBP_HUD.WBP_HUD_C|GetDialoguePanel _interface) 1.0)
  (CallFunction|TypeDialogue))

(fn GenerateChoices
  (params (dialogue :type S%20Dialogue%20Entry%20Structure))
  (Widget|Panel|ClearChildren (Variables|/Game/Widgets/WBP_HUD.WBP_HUD_C|GetChoicePanel (Variables|/Game/Blueprints/Game/BP_LoopHero_GM.BP_LoopHero_GM_C|Getinterface (Variables|Default|GetgameMode))))
  (Utilities|FlowControl|Sequence
    (:then_0
      (if (LocalVariables|GethasBracketChoices)
        (CallFunction|GenerateInputChoice dialogue)))
    (:then_1
      (CallFunction|GenerateButtonChoices dialogue))))

(fn GenerateButtonChoices
  (params (dialogue :type S%20Dialogue%20Entry%20Structure))
  (Widget|SetRenderOpacity (Variables|/Game/Widgets/WBP_HUD.WBP_HUD_C|GetChoicePanel (Variables|/Game/Blueprints/Game/BP_LoopHero_GM.BP_LoopHero_GM_C|Getinterface (Variables|Default|GetgameMode))) 1.0)
  (for _index (range 0 (- (Utilities|Array|Length (.choicestexts dialogue)) 1))
    (bind _returnvalue (UserInterface|CreateWidget (Variables|Default|GetchoicePrefab)))
    (Widget|Panel|AddChild (Variables|/Game/Widgets/WBP_HUD.WBP_HUD_C|GetChoicePanel (Variables|/Game/Blueprints/Game/BP_LoopHero_GM.BP_LoopHero_GM_C|Getinterface (Variables|Default|GetgameMode))) _returnvalue)
    (Variables|/Script/UMG.TextBlock|SetText (Variables|/Game/Widgets/WBP_ChoiceButton.WBP_ChoiceButton_C|GetChoiceText _returnvalue) (Utilities|Text|ToText(String) (Utilities|Array|Get(acopy) (.choicestexts dialogue) _index)))
    (Variables|/Game/Widgets/WBP_ChoiceButton.WBP_ChoiceButton_C|Setindex _returnvalue (Utilities|Array|Get(acopy) (.answersindexes dialogue) _index))
    (EventDispatchers|BindEventtoOnClick _returnvalue (EventDispatchers|CreateEvent (Variables|Default|GetcurrentDialogueComponent) :!event TryDialogue))))

(fn GenerateInputChoice
  (params (dialogue :type S%20Dialogue%20Entry%20Structure)))

(fn SkipDialogue
  (bind _currentspeaker (Variables|Default|GetcurrentSpeaker)
    (:then
      (bind _output_get (LocalVariables|SetisEnd (.dialogueend (Variables|/Game/Blueprints/Dialogue/BPC_Speaker.BPC_Speaker_C|Getdialogue _currentspeaker))))
      (Utilities|FlowControl|Sequence
        (:then_0
          (if _output_get
            (Variables|/Script/UMG.Widget|SetRenderOpacity (Variables|/Game/Widgets/WBP_HUD.WBP_HUD_C|GetDialoguePanel (Variables|/Game/Blueprints/Game/BP_LoopHero_GM.BP_LoopHero_GM_C|Getinterface (Variables|Default|GetgameMode))) 0.0)))
        (:then_1
          (Variables|Default|SetcurrentSpeaker 0)
          (Default|CallOnDialogueSkipped _output_get))))
    (:else)))

(fn TypeDialogue
  (bind _gamemode (Variables|Default|GetgameMode))
  (bind _currentspeaker (Variables|Default|GetcurrentSpeaker))
  (bind _interface (Variables|/Game/Blueprints/Game/BP_LoopHero_GM.BP_LoopHero_GM_C|Getinterface _gamemode))
  (bind _dialogue (Variables|/Game/Blueprints/Dialogue/BPC_Speaker.BPC_Speaker_C|Getdialogue _currentspeaker))
  (bind _skipbutton (Variables|/Game/Widgets/WBP_HUD.WBP_HUD_C|GetSkipButton _interface))
  (Variables|/Script/UMG.TextBlock|SetText (Variables|/Game/Widgets/WBP_HUD.WBP_HUD_C|GetDialogueText (Variables|/Game/Blueprints/Game/BP_LoopHero_GM.BP_LoopHero_GM_C|Getinterface (Variables|Default|GetgameMode))) (Utilities|Text|ToText(String) (Variables|Default|GetcurrentDialogue)))
  (bind _output_get (LocalVariables|SethasChoices (Utilities|Array|IsNotEmpty (Utilities|Struct|BreakSDialogueEntry _dialogue))))
  (if _output_get
    (CallFunction|GenerateChoices _dialogue)
    (Widget|SetRenderOpacity (Variables|/Game/Widgets/WBP_HUD.WBP_HUD_C|GetChoicePanel _interface) 1.0)
    (else
      (Widget|SetVisibility _skipbutton "Visible")
      (Variables|/Script/UMG.Widget|SetRenderOpacity _skipbutton 1.0))))

(fn UpdateText
  (params (displayedLetters :type Integer)))