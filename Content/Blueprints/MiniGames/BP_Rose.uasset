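; BP_Rose is a minigame rose that awards a random amount of Roses the first time the player touches it.
; A capsule overlap by the player pawn fires once, switching two static mesh material slots to Red.
; It then increments the Roses counter on BP_LoopHero_GI one at a time through a short Delay loop, so the total climbs gradually rather than jumping.
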(event OnComponentBeginOverlap(Capsule)
  (params (OverlappedComponent :type Primitive%20Component%20Object%20Reference) (OtherActor :type Actor%20Object%20Reference) (OtherComp :type Primitive%20Component%20Object%20Reference) (OtherBodyIndex :type Integer) (bFromSweep :type Boolean) (SweepResult :type Hit%20Result%20Structure%20%28by%20ref%29))
  (bind _staticmesh (Variables|Default|GetStaticMesh))
  (if (== OtherActor (Game|Player|GetPlayerPawn 0))
    (Utilities|FlowControl|DoOnce false
      (:Completed
        (Rendering|Material|SetMaterial _staticmesh 0 "/Game/Assets/TheOtherOne/red.red")
        (Rendering|Material|SetMaterial _staticmesh 1 "/Game/Assets/TheOtherOne/red.red")
        (bind _asbp_loop_hero_gi (Utilities|Casting|CastToBP_LoopHero_GI (Game|GetGameInstance)))
        (bind _output_get (Variables|Default|SetToAdd (Math|Random|RandomIntegerinRange 37 73)))
        (Math|Integer|CompareInt _output_get :!label _label
          (:>
            (Math|Integer|IncrementInt (Variables|/Game/Blueprints/Game/BP_LoopHero_GI.BP_LoopHero_GI_C|GetRoses _asbp_loop_hero_gi)
              (:%20%20
                (Math|Integer|DecrementInt (Variables|Default|GetToAdd)
                  (:%20%20
                    (Utilities|FlowControl|Delay 0.05)
                    (goto _label)))))))))))

(event EventBeginPlay)

(event Collision|EventActorBeginOverlap
  (params (OtherActor :type Actor%20Object%20Reference)))

(event EventTick
  (params (DeltaSeconds :type Float%20%28single-precision%29)))

(fn ConstructionScript)