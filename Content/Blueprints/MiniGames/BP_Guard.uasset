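; BP_Guard is a minigame guard that wanders near its spawn point and chases the player on sight.
; Each Tick, an unobstructed visibility trace plus a forward dot-product cone check triggers AIMoveTo toward the player.
; Otherwise, after a random Delay, it rechecks and moves to a random navigable point near its spawn anchor.
; That anchor is an inactive particle system spawned at BeginPlay, used only as a location marker.
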(event EventTick
  (params (DeltaSeconds :type Float%20%28single-precision%29))
  (bind _returnvalue (Transformation|GetActorLocation))
  (bind _returnvalue_2 (Transformation|GetActorForwardVector))
  (bind _returnvalue_3 (Game|Player|GetPlayerPawn 0))
  (bind _returnvalue_4 (Transformation|GetActorLocation _returnvalue_3))
  (bind _returnvalue_5 (- _returnvalue_4 _returnvalue))
  (bind _returnvalue_6 (Math|Vector|Normalize _returnvalue_5))
  (bind _returnvalue_7 (Math|Vector|DotProduct _returnvalue_2 _returnvalue_6))
  (bind _returnvalue_8 (> _returnvalue_7 0.75))
  (bind _returnvalue_9 (Collision|LineTraceByChannel _returnvalue _returnvalue_4 "TraceTypeQuery1" false 0 "None"))
  (if _returnvalue_9
    (Utilities|FlowControl|Delay (Math|Random|RandomFloatinRange 4.0 6.0) :!label _label)
    (bind _randomlocation (Class|NavigationSystemV1|GetRandomLocationinNavigableRadius (Transformation|GetWorldLocation (Variables|Default|GetSpawnAnchorLazyFix)) 2.5e+02 0 0))
    (if (or _returnvalue_9 (not _returnvalue_8))
      (AI|AIMoveTo self (.ProjectedLocation (AI|Navigation|ProjectPointtoNavigation _randomlocation 0 0 "0, 0, 0")) 0 5.0 false))
    (elif _returnvalue_8
      (AI|AIMoveTo self "0, 0, 0" (Game|Player|GetPlayerPawn 0) 5.0 false)
      (else
        (goto _label)))))

(event EventBeginPlay
  (bind _returnvalue (Niagara|SpawnSystematLocation "/Niagara/DefaultAssets/DefaultSystem.DefaultSystem" (Transformation|GetActorLocation) "0, 0, 0" "1.000000,1.000000,1.000000" false false))
  (Variables|Default|SetSpawnAnchorLazyFix _returnvalue))

(fn ConstructionScript)