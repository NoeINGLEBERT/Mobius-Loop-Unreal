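; Manager actor for a three-cup shell game that spawns the cups, runs the shuffle and then broadcasts ToggleClick to enable picking.
; BeginPlay makes a random cup's sphere visible, then uses timed delays to raise and lower all cups as a reveal.
; A DoN counter with a delay loop repeats Shuffle before the click broadcast.
; Each Shuffle rotates target indices one step in a random direction, randomizes travel modes and starts each cup's timeline.
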(event EventBeginPlay
  (for (_array_element _array_index) (Utilities|Array|MakeArray (Variables|Default|Get0) (Variables|Default|Get1) (Variables|Default|Get2))
    (bind _returnvalue (Game|SpawnActorfromClass "/Game/Blueprints/MiniGames/BP_Cup.BP_Cup_C" (Math|Transform|MakeTransform (Transformation|GetWorldLocation _array_element) "0, 0, 0" "1.000000,1.000000,1.000000") "Undefined" "MultiplyWithRoot" 0 0))
    (Variables|/Game/Blueprints/MiniGames/BP_Cup.BP_Cup_C|SetIndex _returnvalue _array_index)
    (Variables|/Game/Blueprints/MiniGames/BP_Cup.BP_Cup_C|SetManagerRef _returnvalue self)
    (Utilities|Array|Add (Variables|Default|GetCupArray) _returnvalue)
    (EventDispatchers|BindEventtoToggleClick (EventDispatchers|CreateEvent _returnvalue :!event ToggleClick)))
  (Rendering|SetVisibility (Variables|/Game/Blueprints/MiniGames/BP_Cup.BP_Cup_C|GetSphere (.OutItem (Utilities|Array|Random (Variables|Default|GetCupArray)))) true false)
  (Utilities|FlowControl|Delay 1.0)
  (for _array_element_2 (Variables|Default|GetCupArray)
    (Variables|/Game/Blueprints/MiniGames/BP_Cup.BP_Cup_C|SetTargetIndex _array_element_2 (Variables|/Game/Blueprints/MiniGames/BP_Cup.BP_Cup_C|GetIndex _array_element_2))
    (Variables|/Game/Blueprints/MiniGames/BP_Cup.BP_Cup_C|SetTravelMode _array_element_2 0)
    (Variables|/Game/Blueprints/MiniGames/BP_Cup.BP_Cup_C|SetTargetIsUp _array_element_2 true)
    (Default|StartTimeline _array_element_2))
  (Utilities|FlowControl|Delay 2.0)
  (for _array_element_3 (Variables|Default|GetCupArray)
    (Variables|/Game/Blueprints/MiniGames/BP_Cup.BP_Cup_C|SetTargetIsUp _array_element_3 false)
    (Default|StartTimeline _array_element_3))
  (Utilities|FlowControl|Delay 1.0)
  (bind _counter (Utilities|FlowControl|DoN 10 :!label _label)
    (:Exit
      (if (== _counter 10)
        (Default|CallToggleClick true)
        (else
          (CallFunction|Shuffle)
          (Utilities|FlowControl|Delay 0.3)
          (goto _label))))))

(fn ConstructionScript)

(fn Shuffle
  (bind _cuparray (Variables|Default|GetCupArray))
  (bind _returnvalue (Utilities|Array|Length _cuparray))
  (LocalVariables|SetShuffleDir (.OutItem (Utilities|Array|Random (Utilities|Array|MakeArray 1 -1))))
  (Utilities|Array|Shuffle (LocalVariables|GetTravMode))
  (for (_array_element _array_index) _cuparray
    (Variables|/Game/Blueprints/MiniGames/BP_Cup.BP_Cup_C|SetTargetIndex _array_element (Math|Integer|%(Integer) (+ (+ (Variables|/Game/Blueprints/MiniGames/BP_Cup.BP_Cup_C|GetIndex _array_element) (LocalVariables|GetShuffleDir)) _returnvalue) _returnvalue))
    (Variables|/Game/Blueprints/MiniGames/BP_Cup.BP_Cup_C|SetTravelMode _array_element (Utilities|Array|Get(acopy) (LocalVariables|GetTravMode) _array_index))
    (Default|StartTimeline _array_element)))