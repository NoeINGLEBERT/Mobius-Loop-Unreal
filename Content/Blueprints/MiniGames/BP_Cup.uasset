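; BP_Cup is a cup actor in a minigame that swaps between three positions held by its manager, apparently for a shell-game shuffle.
; StartTimeline records the current index, adopts TargetIndex, then plays a sped-up timeline that lerps the cup between those two positions.
; A second timeline track, scaled by TravelMode, offsets the path along the actor's right vector, so the cup can swing sideways during the move.
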(event Custom|StartTimeline
  (bind _managerref (Variables|Default|GetManagerRef))
  (bind _0 (Variables|/Game/Blueprints/MiniGames/BP_CupManager.BP_CupManager_C|Get0 _managerref))
  (bind _1 (Variables|/Game/Blueprints/MiniGames/BP_CupManager.BP_CupManager_C|Get1 _managerref))
  (bind _2 (Variables|/Game/Blueprints/MiniGames/BP_CupManager.BP_CupManager_C|Get2 _managerref))
  (bind _array (Utilities|Array|MakeArray _0 _1 _2))
  (Variables|Default|SetStartIndex (Variables|Default|GetIndex))
  (Variables|Default|SetIndex (Variables|Default|GetTargetIndex))
  (bind (_direction _alpha _axis) (Timeline|Timeline PlayFromStart)
    (:Update
      (Transformation|SetActorLocation (+ (Math|Vector|Lerp(Vector) (Transformation|GetWorldLocation (Utilities|Array|Get(acopy) _array (Variables|Default|GetStartIndex))) (Transformation|GetWorldLocation (Utilities|Array|Get(acopy) _array (Variables|Default|GetTargetIndex))) _alpha) (* (Transformation|GetActorRightVector) (* (* _axis (Variables|Default|GetTravelMode)) 8e+01))) false false))))

(event EventBeginPlay
  (Components|Timeline|SetPlayRate (Variables|Default|GetTimeline) 4.0))

(event Collision|EventActorBeginOverlap
  (params (OtherActor :type Actor%20Object%20Reference)))

(event EventTick
  (params (DeltaSeconds :type Float%20%28single-precision%29)))

(fn ConstructionScript)